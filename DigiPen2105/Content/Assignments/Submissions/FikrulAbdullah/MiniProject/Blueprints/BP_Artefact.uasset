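; Collectible artefact Blueprint, built on an activatable parent, that vanishes with a star effect when activated.
; On BeginPlay it sets its text render to a success message.
; Activation runs the parent logic, hides the mesh, disables mesh and trigger collisions, sets CheckDone, stops animation and spawns the emitter below the mesh.
; A timeline update bobs and spins the mesh; only its Stop input is wired here.
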(event Custom|Stop_Anim
  (bind _basic_mesh (Variables|Default|GetBasic_Mesh))
  ;[1 1 1] Bouncy Bouncy
  (bind _newtrack_0 (Timeline|Timeline_0 Stop)
    (:Update
      (Transformation|SetRelativeLocation _basic_mesh (Math|Vector|Lerp(Vector) (Variables|Default|GetCenterLocation) (Variables|Default|GetMaxLocation) _newtrack_0) false false)
      (Transformation|AddLocalRotation _basic_mesh "0,1.000000, 0" false false))))

(event Custom|HideMeshAndRemoveCollisions
  (bind _basic_mesh (Variables|Default|GetBasic_Mesh))
  ;[1 1 1] Hide Mesh and Remova All Collisions
  (Development|SetHiddeninGame _basic_mesh true false)
  (Collision|SetCollisionEnabled _basic_mesh "NoCollision")
  (Collision|SetCollisionEnabled (Variables|Default|GetDetectActivation) "NoCollision")
  (Collision|SetCollisionEnabled (Variables|Default|GetHelp_Trigger) "NoCollision")
  (Variables|Default|SetCheckDone true))

(event EventBeginPlay
  (|CallParentFunction)
  (Rendering|Components|TextRender|SetText (Variables|Default|GetTextRender) (Variables|Default|GetText_MessageSuccess_Line1)))

(event EventObjectActivated
  (params (WhoActivatedMe? :type Actor%20Object%20Reference))
  (bind _basic_mesh (Variables|Default|GetBasic_Mesh))
  (bind _returnvalue (Transformation|GetWorldLocation _basic_mesh))
  (|CallParentFunction WhoActivatedMe?)
  (CallFunction|HideMeshandRemoveCollisions)
  (CallFunction|StopAnim)
  (Effects|SpawnEmitteratLocation "/Game/DigiPen/07_Particles/P_Star_Icon.P_Star_Icon" (Math|Vector|MakeVector (.x _returnvalue) (.y _returnvalue) (- (.z _returnvalue) 1.5e+02))))

(fn ConstructionScript
  (|CallParentFunction))