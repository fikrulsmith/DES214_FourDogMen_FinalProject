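; BP_ArtefactDoor is an activatable door, built on a parent class, that slides upward once CanOpenDoor is true.
; BeginPlay stops the bounce timeline and sets the text render, while activation of an openable door spawns a star effect below the mesh.
; UpdateDoor stores a target above the mesh, which Tick eases toward with VInterpTo.
; Nothing here calls UpdateDoor, and the nodes that set CanOpenDoor or call HideMeshAndRemoveCollisions are disconnected.
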(event Custom|Stop_Anim
  ;[1 1 1] Bouncy Bouncy
  (bind _newtrack_0 (Timeline|Timeline_0 Stop)
    (:Update
      (Transformation|SetRelativeLocation (Variables|Default|GetBasic_Mesh) (Math|Vector|Lerp(Vector) (Variables|Default|GetCenterLocation) (Variables|Default|GetMaxLocation) _newtrack_0) false false))))

(event Custom|Update%20Door
  (Variables|Default|SetNewVar_0 (+ (Transformation|GetWorldLocation (Variables|Default|GetBasic_Mesh)) "0, 0,300.000000")))

(event Custom|HideMeshAndRemoveCollisions
  (bind _basic_mesh (Variables|Default|GetBasic_Mesh))
  ;[1 1 1] Hide Mesh and Remova All Collisions
  (Development|SetHiddeninGame _basic_mesh true false)
  (Collision|SetCollisionEnabled _basic_mesh "NoCollision")
  (Collision|SetCollisionEnabled (Variables|Default|GetDetectActivation) "NoCollision")
  (Collision|SetCollisionEnabled (Variables|Default|GetHelp_Trigger) "NoCollision"))

(event EventBeginPlay
  (|CallParentFunction)
  (CallFunction|StopAnim)
  (Rendering|Components|TextRender|SetText (Variables|Default|GetTextRender) (Variables|Default|GetText_MessageSuccess_Line1)))

(event EventObjectActivated
  (params (WhoActivatedMe? :type Actor%20Object%20Reference))
  (bind _basic_mesh (Variables|Default|GetBasic_Mesh))
  (bind _returnvalue (Transformation|GetWorldLocation _basic_mesh))
  (|CallParentFunction WhoActivatedMe?)
  (if (Variables|Default|GetCanOpenDoor)
    (CallFunction|StopAnim)
    (Effects|SpawnEmitteratLocation "/Game/DigiPen/07_Particles/P_Star_Icon.P_Star_Icon" (Math|Vector|MakeVector (.x _returnvalue) (.y _returnvalue) (- (.z _returnvalue) 1.5e+02)))))

(event EventTick
  (params (DeltaSeconds :type Float%20%28single-precision%29))
  (if (Variables|Default|GetCanOpenDoor)
    (Transformation|SetWorldLocation (Variables|Default|GetBasic_Mesh) (Math|Interpolation|VInterpTo (Transformation|GetWorldLocation (Variables|Default|GetBasic_Mesh)) (Variables|Default|GetNewVar_0) DeltaSeconds 5.0) false false)))

(fn ConstructionScript
  (|CallParentFunction))