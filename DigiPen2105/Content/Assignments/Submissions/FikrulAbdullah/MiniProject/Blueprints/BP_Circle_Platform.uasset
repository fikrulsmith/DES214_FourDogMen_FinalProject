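; Circle platform actor that drops and rises between two reference actors and can shake its mesh.
; External calls to PlatformDrop and PlatformRise play or reverse one timeline, lerping the actor from Start to End and updating dropped/risen state flags on finish.
; While IsVibrating is set, each VibratePlatform call offsets the mesh by a per-axis time-based sine wave around a position cached on the first call.
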(event Custom|PlatformDrop
  ;[1 1 1] PlatformRise/Drop
  (Variables|Default|SetHasRisen false)
  (Variables|Default|SetIsDropping true)
  (bind _newtrack_0 (Timeline|CircleTimeline Play)
    (:Update
      (Transformation|SetActorLocation self (Math|Vector|Lerp(Vector) (Transformation|GetActorLocation (Variables|TargetElements|GetStart)) (Transformation|GetActorLocation (Variables|TargetElements|GetEnd)) _newtrack_0) false false))
    (:Finished
      (if (Variables|Default|GetIsDropping)
        (Variables|Default|SetHasDropped true)
        (Variables|Default|SetIsDropping false)
        (elif (Variables|Default|GetIsRising)
          (Variables|Default|SetHasRisen true)
          (Variables|Default|SetIsRising false))))))

(event Custom|PlatformRise
  ;[1 1 1] PlatformRise/Drop
  (Variables|Default|SetHasDropped false)
  (Variables|Default|SetIsRising true)
  (bind _newtrack_0 (Timeline|CircleTimeline Reverse)
    (:Update
      (Transformation|SetActorLocation self (Math|Vector|Lerp(Vector) (Transformation|GetActorLocation (Variables|TargetElements|GetStart)) (Transformation|GetActorLocation (Variables|TargetElements|GetEnd)) _newtrack_0) false false))
    (:Finished
      (if (Variables|Default|GetIsDropping)
        (Variables|Default|SetHasDropped true)
        (Variables|Default|SetIsDropping false)
        (elif (Variables|Default|GetIsRising)
          (Variables|Default|SetHasRisen true)
          (Variables|Default|SetIsRising false))))))

(event Custom|VibratePlatform
  (bind _returnvalue (Utilities|Time|GetGameTimeinSeconds))
  (bind _staticmeshcomponent (Variables|Default|GetStaticMeshComponent))
  (bind _amplitude (Variables|Default|GetAmplitude))
  (bind _frequency (Variables|Default|GetFrequency))
  (bind _shakexyz (Variables|Default|GetShakeXYZ))
  (bind _returnvalue_2 (* _frequency _returnvalue))
  (bind (_x _y _z) (Math|Vector|BreakVector _shakexyz))
  (bind _returnvalue_3 (Math|Trig|Sin(Radians) _returnvalue_2))
  (bind _returnvalue_4 (* _amplitude _returnvalue_3))
  ;[1 1 1] Vibrating Logic
  (if (Variables|Default|GetIsVibrating)
    (Utilities|FlowControl|Sequence
      (:then_0
        (if (Variables|Default|GetIsPositionSet)
          (Transformation|SetWorldLocation _staticmeshcomponent (+ (Math|Vector|MakeVector (* _returnvalue_4 _x) (* _y _returnvalue_4) (* _z _returnvalue_4)) (Variables|Default|GetOriginalPosition)) false false)
          (else
            (Variables|Default|SetOriginalPosition (Transformation|GetWorldLocation _staticmeshcomponent))
            (Variables|Default|SetIsPositionSet true)))))))

(event EventBeginPlay)

(event Collision|EventActorBeginOverlap
  (params (OtherActor :type Actor%20Object%20Reference)))

(fn ConstructionScript)