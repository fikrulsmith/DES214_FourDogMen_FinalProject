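; Clock actor whose left and right hit buttons turn a glass piece in quarter steps, lighting one of four shapes.
; Rotation finds its target by turning and undoing, steps a wrapping PositionIndex and clears shape flags; Tick eases the glass there with RInterpTo.
; Tick also runs Coordinator, which re-binds button hits and sets the indexed shape while idle, then swaps Clock materials to match the flags.
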(event Custom|RInterpolate
  (bind _clocklightupglass (Variables|Default|GetClockLightUpGlass))
  ;[1 1 1] Rotate Interpolation Logic
  (if (Variables|Default|GetIsMoving)
    (Transformation|SetWorldRotation (Variables|Default|GetClockLightUpGlass) (Math|Interpolation|RInterpTo (Transformation|GetWorldRotation _clocklightupglass) (Variables|Default|GetTarget) (Variables|Default|GetDelta%20Seconds) 2.5) false false)
    (if (Math|Rotator|Equal(Rotator) (Transformation|GetWorldRotation _clocklightupglass) (Variables|Default|GetTarget) 0.2)
      (Variables|Default|SetIsMoving false))))

(event Custom|TurnOnTriangle
  ;[1 1 1] Change Shape's Material Logic
  (Rendering|Material|SetMaterial (Variables|Default|GetClock) 1 "/Game/DigiPen/06_Materials/BaseMaterial/BaseMaterial_Inst_GreenEmissive.BaseMaterial_Inst_GreenEmissive"))

(event Custom|TurnOffTriangle
  ;[1 1 1] Change Shape's Material Logic
  (Rendering|Material|SetMaterial (Variables|Default|GetClock) 1 "/Game/DigiPen/06_Materials/BaseMaterial/BaseMaterial_Inst_Z_006115FF.BaseMaterial_Inst_Z_006115FF"))

(event Custom|TurnOnSquare
  ;[1 1 1] Change Shape's Material Logic
  (Rendering|Material|SetMaterial (Variables|Default|GetClock) 2 "/Game/DigiPen/06_Materials/BaseMaterial/BaseMaterial_Inst_WhiteEmissive2.BaseMaterial_Inst_WhiteEmissive2"))

(event Custom|TurnOffSquare
  ;[1 1 1] Change Shape's Material Logic
  (Rendering|Material|SetMaterial (Variables|Default|GetClock) 2 "/Game/DigiPen/06_Materials/BaseMaterial/BaseMaterial_Inst_Blue.BaseMaterial_Inst_Blue"))

(event Custom|RotateRight
  (bind _clocklightupglass (Variables|Default|GetClockLightUpGlass))
  ;[1 1 1] Glass_Rotation_Logic
  (if (not (Variables|Default|GetIsMoving))
    (Transformation|AddLocalRotation _clocklightupglass "0,90.000000, 0" false false)
    (Variables|Default|SetTarget (Transformation|GetWorldRotation _clocklightupglass))
    (Transformation|AddLocalRotation (Variables|Default|GetClockLightUpGlass) "0,-90.000000, 0" false false)
    (Variables|Default|SetIsMoving true)
    (CallFunction|ResetShapes)
    (if (== (Variables|Default|GetPositionIndex) 4)
      (Variables|Default|SetPositionIndex 1)
      (else
        (Math|Integer|IncrementInt (Variables|Default|GetPositionIndex))))))

(event Custom|TurnOnCircle
  ;[1 1 1] Change Shape's Material Logic
  (Rendering|Material|SetMaterial (Variables|Default|GetClock) 3 "/Game/DigiPen/06_Materials/BaseMaterial/BaseMaterial_Inst_YellowGlow_Intense.BaseMaterial_Inst_YellowGlow_Intense"))

(event Custom|TurnOffCircle
  ;[1 1 1] Change Shape's Material Logic
  (Rendering|Material|SetMaterial (Variables|Default|GetClock) 3 "/Game/DigiPen/06_Materials/BaseMaterial/BaseMaterial_Inst_Z_FF8A01FF.BaseMaterial_Inst_Z_FF8A01FF"))

(event Custom|TurnOnPentagon
  ;[1 1 1] Change Shape's Material Logic
  (Rendering|Material|SetMaterial (Variables|Default|GetClock) 4 "/Game/DigiPen/06_Materials/BaseMaterial/BaseMaterial_Inst_RedEmissive.BaseMaterial_Inst_RedEmissive"))

(event Custom|TurnOffPentagon
  ;[1 1 1] Change Shape's Material Logic
  (Rendering|Material|SetMaterial (Variables|Default|GetClock) 4 "/Game/DigiPen/06_Materials/BaseMaterial/BaseMaterial_Inst_Z_FF000000_R100.BaseMaterial_Inst_Z_FF000000_R100"))

(event Custom|Coordinator
  ;[1 1 1] Coordinator
  (if (Variables|Default|GetIsMoving)
    _
    (else
      (CallFunction|ButtonRightHit)
      (CallFunction|SetShape)))
  (if (Variables|Default|GetIsMoving)
    _
    (else
      (CallFunction|ButtonLeftHit)
      (CallFunction|SetShape)))
  (if (Variables|Default|GetIsTriangle)
    (CallFunction|TurnonTriangle)
    (else
      (CallFunction|TurnOffTriangle)))
  (if (Variables|Default|GetIsSquare)
    (CallFunction|TurnonSquare)
    (else
      (CallFunction|TurnOffSquare)))
  (if (Variables|Default|GetIsPentagon)
    (CallFunction|TurnonPentagon)
    (else
      (CallFunction|TurnOffPentagon)))
  (if (Variables|Default|GetIsCircle)
    (CallFunction|TurnonCircle)
    (else
      (CallFunction|TurnOffCircle))))

(event Custom|SetShape
  ;[1 1 1] Set/Reset Shapes
  (switch int (Variables|Default|GetPositionIndex)
    (:1
      (Variables|Default|SetIsTriangle true))
    (:2
      (Variables|Default|SetIsSquare true))
    (:3
      (Variables|Default|SetIsPentagon true))
    (:4
      (Variables|Default|SetIsCircle true))))

(event Custom|RotateLeft
  (bind _clocklightupglass (Variables|Default|GetClockLightUpGlass))
  ;[1 1 1] Glass_Rotation_Logic
  (if (not (Variables|Default|GetIsMoving))
    (Transformation|AddLocalRotation _clocklightupglass "0,-90.000000, 0" false false)
    (Variables|Default|SetTarget (Transformation|GetWorldRotation _clocklightupglass))
    (Transformation|AddLocalRotation (Variables|Default|GetClockLightUpGlass) "0,90.000000, 0" false false)
    (Variables|Default|SetIsMoving true)
    (CallFunction|ResetShapes)
    (if (== (Variables|Default|GetPositionIndex) 1)
      (Variables|Default|SetPositionIndex 4)
      (else
        (Math|Integer|DecrementInt (Variables|Default|GetPositionIndex))))))

(event Custom|ResetShapes
  ;[1 1 1] Set/Reset Shapes
  (Variables|Default|SetIsTriangle false)
  (Variables|Default|SetIsSquare false)
  (Variables|Default|SetIsCircle false)
  (Variables|Default|SetIsPentagon false))

(event Custom|DetectRightHit
  (params (HitComponent :type Primitive%20Component%20Object%20Reference) (OtherActor :type Actor%20Object%20Reference) (OtherComp :type Primitive%20Component%20Object%20Reference) (NormalImpulse :type Vector) (Hit :type Hit%20Result%20Structure%20%28by%20ref%29))
  ;[1 1 1] Button Logic
  (CallFunction|RotateRight))

(event Custom|ButtonRightHit
  ;[1 1 1] Button Logic
  (Collision|AssignOnComponentHit (Variables|Default|GetClockButtonRight) (delegate Custom|DetectRightHit)))

(event Custom|ButtonLeftHit
  ;[1 1 1] Button Logic
  (Collision|BindEventtoOnComponentHit (Variables|Default|GetClockButton_Left) (delegate Custom|DetectLeftHit)))

(event Custom|DetectLeftHit
  (params (HitComponent :type Primitive%20Component%20Object%20Reference) (OtherActor :type Actor%20Object%20Reference) (OtherComp :type Primitive%20Component%20Object%20Reference) (NormalImpulse :type Vector) (Hit :type Hit%20Result%20Structure%20%28by%20ref%29))
  ;[1 1 1] Button Logic
  (CallFunction|RotateLeft))

(event EventBeginPlay)

(event EventTick
  (params (DeltaSeconds :type Float%20%28single-precision%29))
  (Variables|Default|SetDelta%20Seconds DeltaSeconds)
  (CallFunction|RInterpolate)
  (CallFunction|Coordinator))

(fn ConstructionScript)