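; BP_DEATHDROP is a death-drop trigger that sends the first-person player back to a spawn point.
; When DPChar_C_TrueFirstPerson overlaps its Cube, it shows a blood overlay, moves the character to SpawnPoint's transform, then immediately starts the overlay's fade-out.
; The Blood_UI widget is created once at BeginPlay, and ShowBlood uses a DoOnce to guard AddToViewport, resetting it after calling FadeOut.
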(event OnComponentBeginOverlap(Cube)
  (params (OverlappedComponent :type Primitive%20Component%20Object%20Reference) (OtherActor :type Actor%20Object%20Reference) (OtherComp :type Primitive%20Component%20Object%20Reference) (OtherBodyIndex :type Integer) (bFromSweep :type Boolean) (SweepResult :type Hit%20Result%20Structure%20%28by%20ref%29))
  (Utilities|Casting|CastToDPChar_C_TrueFirstPerson OtherActor)
  (CallFunction|ShowBlood true)
  (Transformation|SetActorTransform OtherActor (Transformation|GetActorTransform (Variables|Default|GetSpawnPoint)))
  (CallFunction|ShowBlood false))

(event EventBeginPlay
  (bind _returnvalue (UserInterface|CreateWidget "/Game/Assignments/Submissions/FikrulAbdullah/MiniProject/UI/Blood_UI.Blood_UI_C"))
  (Variables|Default|SetBLOOD_REF _returnvalue))

(event Collision|EventActorBeginOverlap
  (params (OtherActor :type Actor%20Object%20Reference)))

(event EventTick
  (params (DeltaSeconds :type Float%20%28single-precision%29)))

(fn ConstructionScript)

(fn ShowBlood
  (params (AddToScreen :type Boolean))
  (bind _blood_ref (Variables|Default|GetBLOOD_REF))
  (if AddToScreen
    (Utilities|FlowControl|DoOnce false :!label _label
      (:Completed
        (UserInterface|Viewport|AddtoViewport _blood_ref 0)))
    (else
      (Default|FadeOut _blood_ref)
      (goto _label Reset))))