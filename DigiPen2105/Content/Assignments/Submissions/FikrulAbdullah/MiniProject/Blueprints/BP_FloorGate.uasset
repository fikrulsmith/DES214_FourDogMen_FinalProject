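; BP_FloorGate is a gate actor whose FloorGate component slides 300 units along world Y to open.
; The OpenGate event stores that target once, offset from the current world position, through a DoOnce.
; While the Open flag is true, Tick eases the component toward the target with VInterpTo; nothing in this graph sets that flag.
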(event Custom|OpenGate
  (Utilities|FlowControl|DoOnce false
    (:Completed
      (Variables|Default|SetOpenVec (+ (Transformation|GetWorldLocation (Variables|Default|GetFloorGate)) "0.000000,300.000000,0.000000")))))

(event EventTick
  (params (DeltaSeconds :type Float%20%28single-precision%29))
  (if (Variables|Default|GetOpen)
    (Transformation|SetWorldLocation (Variables|Default|GetFloorGate) (Math|Interpolation|VInterpTo (Transformation|GetWorldLocation (Variables|Default|GetFloorGate)) (Variables|Default|GetOpenVec) DeltaSeconds 5.0) false false)))

(fn ConstructionScript)