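; Base interactable object that reports its activation by a character and shows hint text when sensed.
; Interacting stores the activating character, fires an activation dispatcher, pushes success text to the HUD's mission update widget and disables the hint.
; Sensing toggles the player's Component_HintText.
; Custom depth stencil highlight events exist, but their setup and calls are disconnected, and the trigger overlap logic is deprecated.
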(event OnComponentBeginOverlap(Help_Trigger)
  (params (OverlappedComponent :type Primitive%20Component%20Object%20Reference) (OtherActor :type Actor%20Object%20Reference) (OtherComp :type Primitive%20Component%20Object%20Reference) (OtherBodyIndex :type Integer) (bFromSweep :type Boolean) (SweepResult :type Hit%20Result%20Structure%20%28by%20ref%29))
  ;[1 1 1] DEPRECATED, MOved to other compoments
  ;;[1 0 0] DEPRECATED
  (bind _ascharacter (Utilities|Casting|CastToCharacter OtherActor))
  (if (Pawn|IsPlayerControlled _ascharacter)
    _))

(event OnComponentEndOverlap(Help_Trigger)
  (params (OverlappedComponent :type Primitive%20Component%20Object%20Reference) (OtherActor :type Actor%20Object%20Reference) (OtherComp :type Primitive%20Component%20Object%20Reference) (OtherBodyIndex :type Integer))
  ;[1 1 1] DEPRECATED, MOved to other compoments
  ;;[1 0 0] DEPRECATED
)

(event Custom|ObjectActivated
  (params (WhoActivatedMe? :type Actor%20Object%20Reference))
  ;[1 1 1] Object Activated Logic
  (bind _ascharacter (Utilities|Casting|CastToCharacter WhoActivatedMe?))
  (Variables|Default|SetWhoActivatedMe? _ascharacter)
  (CallFunction|UpdateUIAfterActivated)
  (Default|CallDispatchObjectActivated))

(event Custom|Disable_HelpText
  ;[1 1 1] Help Text
  (Variables|Default|SetbDisableHelpText? true)
  (if (Variables|Default|GetbHelpTextON?)
    (Default|HIDEHintText (Variables|Default|GetPlayerHintWidget))))

(event Custom|Enable_HelpText
  ;[1 1 1] Help Text
  (Variables|Default|SetbDisableHelpText? false))

(event Custom|Activate_PostProcess
  ;[1 1 1] DEPRECATED, MOved to other compoments
  ;;[1 1 1] Activate/Deactivate Post Process for main Mesh
  (Rendering|SetCustomDepthStencilValue (Variables|Default|GetBasic_Mesh) 1)
  ;;[1 1 1] Activate/Deactivate Post Process ofr Child Meshes
  (for _array_element (Variables|Default|GetList%20of%20Static%20Mesh%20Components)
    (Utilities|IsValid _array_element
      (:Is%20Valid
        (Rendering|SetCustomDepthStencilValue _array_element 1)))))

(event Custom|Deactivate_PostProcess
  ;[1 1 1] DEPRECATED, MOved to other compoments
  ;;[1 1 1] Activate/Deactivate Post Process for main Mesh
  (Rendering|SetCustomDepthStencilValue (Variables|Default|GetBasic_Mesh) 0)
  ;;[1 1 1] Activate/Deactivate Post Process ofr Child Meshes
  (for _array_element (Variables|Default|GetList%20of%20Static%20Mesh%20Components)
    (Utilities|IsValid _array_element
      (:Is%20Valid
        (Rendering|SetCustomDepthStencilValue _array_element 0)))))

(event Custom|Sensed_ON
  (bind _returnvalue (Game|GetPlayerCharacter 0))
  (bind _returnvalue_2 (Actor|GetComponentbyClass _returnvalue "/Game/DigiPen/00_Player/Components/Component_HintText/Component_HintText.Component_HintText_C"))
  ;[1 1 1] Help Text
  (if (not (Variables|Default|GetbDisableHelpText?))
    (Utilities|IsValid _returnvalue_2
      (:Is%20Valid
        (Variables|Default|SetPlayerHintWidget _returnvalue_2)
        (Variables|Default|SetbHelpTextON? true)
        (Default|SHOWHintText (Variables|Default|GetPlayerHintWidget))))))

(event Custom|Sensed_OFF
  ;[1 1 1] Help Text
  (if (Variables|Default|GetbHelpTextON?)
    (Default|HIDEHintText (Variables|Default|GetPlayerHintWidget))))

(event Custom|UpdateUI_After_Activated
  (bind _text_messagesuccess_line1 (Variables|Default|GetText_MessageSuccess_Line1))
  (bind _text_messagesuccess_line2 (Variables|Default|GetText_MessageSuccess_Line2))
  (bind _null_text (Variables|Default|GetNull_Text))
  ;[1 1 1] Show Activated Message on UI (Hacky solution)
  (bind _asplayer_controller (Utilities|Casting|CastToPlayerController (Pawn|GetController (Variables|Default|GetWhoActivatedMe?))))
  (bind _asdp_hud (Utilities|Casting|CastToDP_HUD (HUD|GetHUD _asplayer_controller)))
  (Utilities|IsValid (Variables|/Game/DigiPen/00_Player/UI/DP_HUD.DP_HUD_C|GetHeadsUpDisplay _asdp_hud)
    (:Is%20Valid
      (if (not (and (Utilities|Enum|Equal(Enum) _text_messagesuccess_line1 _null_text) (Utilities|Enum|Equal(Enum) _text_messagesuccess_line2 _null_text)))
        (Default|UIMissionUpdateSHOW (Variables|/Game/DigiPen/00_Player/UI/DP_HUDWidget_Main.DP_HUDWidget_Main_C|GetDP_HUDWidget_MissionUpdate (Variables|/Game/DigiPen/00_Player/UI/DP_HUD.DP_HUD_C|GetHeadsUpDisplay _asdp_hud)) _text_messagesuccess_line1 _text_messagesuccess_line2)))))

(event EventBeginPlay)

(event EventInteractable
  (params (WhoActivatedThis? :type Actor%20Object%20Reference))
  ;[1 1 1] Interface Logic
  (CallFunction|ObjectActivated WhoActivatedThis?)
  (CallFunction|DisableHelpText))

(event EventInteractableSensed
  (params (IsInRange :type Boolean))
  ;[1 1 1] Interface Logic
  (if IsInRange
    (CallFunction|SensedON)
    (else
      (CallFunction|SensedOFF))))

(fn ConstructionScript)

(fn QueryInteractMessage
  (return (Variables|Default|GetText_MessageSuccess_Line1) (Variables|Default|GetText_MessageSuccess_Line2)))

(fn QueryInteractState
  (return (Variables|Default|GetDONT_Interact?)))