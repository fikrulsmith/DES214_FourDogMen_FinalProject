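; Swinging obstacle that sends the first-person player back to a spawn point when its box collision overlaps them.
; BeginPlay stores the start rotation and a roll-offset target, and creates a hidden blood overlay widget.
; A Delay on Tick replays a timeline every few seconds, lerping the actor's rotation between the two.
; On overlap, the player teleports to SpawnLoc while Respawn shows the overlay and immediately starts its fade-out.
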(event OnComponentBeginOverlap(PlayerCollisionForBox)
  (params (OverlappedComponent :type Primitive%20Component%20Object%20Reference) (OtherActor :type Actor%20Object%20Reference) (OtherComp :type Primitive%20Component%20Object%20Reference) (OtherBodyIndex :type Integer) (bFromSweep :type Boolean) (SweepResult :type Hit%20Result%20Structure%20%28by%20ref%29))
  ;[1 1 1] PlayerDeath
  (Utilities|Casting|CastToDPChar_C_TrueFirstPerson OtherActor)
  (CallFunction|Respawn true)
  (Transformation|SetActorTransform OtherActor (Transformation|GetActorTransform (Variables|CustomizableData|GetSpawnLoc)))
  (CallFunction|Respawn false))

(event EventBeginPlay
  (bind _returnvalue (Transformation|GetActorRotation))
  (bind (_roll _pitch _yaw) (Math|Rotator|BreakRotator _returnvalue))
  ;[1 1 1] Initialization
  (Variables|Default|SetCurrentPosition _returnvalue)
  (Variables|Default|SetSwingTo (Math|Rotator|MakeRotator (+ _roll (Variables|CustomizableData|GetSwingDistanceInDegrees)) _pitch _yaw))
  (bind _returnvalue_2 (UserInterface|CreateWidget "/Game/Assignments/Submissions/FikrulAbdullah/MiniProject/UI/Blood_UI.Blood_UI_C"))
  (Variables|Default|SetUI_Ref _returnvalue_2)
  (Widget|SetVisibility (Variables|Default|GetUI_Ref) "Hidden")
  (UserInterface|Viewport|AddtoViewport (Variables|Default|GetUI_Ref) 0))

(event Collision|EventActorBeginOverlap
  (params (OtherActor :type Actor%20Object%20Reference)))

(event EventTick
  (params (DeltaSeconds :type Float%20%28single-precision%29))
  ;[1 1 1] Swinging Logic
  (Utilities|FlowControl|Delay 4.0)
  (bind _swingtrack (Timeline|SwingTimeline PlayFromStart)
    (:Update
      (Transformation|SetActorRotation (Math|Rotator|Lerp(Rotator) (Variables|Default|GetCurrentPosition) (Variables|Default|GetSwingTo) _swingtrack)))))

(fn ConstructionScript)

(fn Respawn
  (params (AddToScreen :type Boolean))
  (bind _ui_ref (Variables|Default|GetUI_Ref))
  (if AddToScreen
    (Widget|SetVisibility _ui_ref "Visible")
    (else
      (Default|FadeOut _ui_ref))))