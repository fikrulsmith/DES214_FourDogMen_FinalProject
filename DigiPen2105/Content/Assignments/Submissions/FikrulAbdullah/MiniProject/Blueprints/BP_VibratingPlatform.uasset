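; BP_VibratingPlatform is a platform actor that shakes its Pillar component for a set duration when SetVibrate is called.
; Tick caches the Pillar's world location, then offsets it by a game-time sine wave using amplitude, frequency and a per-axis ShakeXYZ scale.
; On timeout it resets its state and calls the PlatformVibrated dispatcher, without restoring the cached location.
; OffVibrate only clears the Vibrate flag.
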(event Custom|SetVibrate
  (Variables|Default|Setvibrate true))

(event Custom|OffVibrate
  (Variables|Default|Setvibrate false))

(event EventBeginPlay)

(event Collision|EventActorBeginOverlap
  (params (OtherActor :type Actor%20Object%20Reference)))

(event EventTick
  (params (DeltaSeconds :type Float%20%28single-precision%29))
  (bind _returnvalue (Utilities|Time|GetGameTimeinSeconds))
  (bind _pillar (Variables|Components|GetPillar))
  (bind _frequency (Variables|Default|GetFrequency))
  (bind _amplitude (Variables|Default|Getamplitude))
  (bind _shakexyz (Variables|Default|GetShakeXYZ))
  (bind _returnvalue_2 (* _frequency _returnvalue))
  (bind (_x _y _z) (Math|Vector|BreakVector _shakexyz))
  (bind _returnvalue_3 (Math|Trig|Sin(Radians) _returnvalue_2))
  (bind _returnvalue_4 (* _amplitude _returnvalue_3))
  (if (Variables|Default|Getvibrate)
    (Utilities|FlowControl|Sequence
      (:then_0
        (if (not (Variables|Default|GetPositionSet))
          (Variables|Default|SetOriginalPosition (Transformation|GetWorldLocation _pillar))
          (Variables|Default|SetPositionSet true)))
      (:then_1
        (Variables|Default|SetvibrateTimer (+ (Variables|Default|GetvibrateTimer) DeltaSeconds))
        (if (<= (Variables|Default|GetvibrateTimer) (Variables|Default|GetVibrateDuration))
          (Transformation|SetWorldLocation _pillar (+ (Math|Vector|MakeVector (* _returnvalue_4 _x) (* _y _returnvalue_4) (* _z _returnvalue_4)) (Variables|Default|GetOriginalPosition)) false false)
          (else
            (Variables|Default|SetvibrateTimer 0.0)
            (Variables|Default|Setvibrate false)
            (Variables|Default|SetPositionSet false)
            (Default|CallPlatformVibrated)))))))

(fn ConstructionScript)