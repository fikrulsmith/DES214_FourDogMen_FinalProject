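; VibratingPlatformBP is a platform Blueprint that continuously shakes its Pillar component back and forth.
; BeginPlay stores the Pillar's world location, and Tick offsets it from there with a sine of game time scaled by Amplitude and Frequency.
; ShakeXYZ scales the oscillation on X and Y, but its Z value is added as a constant offset without the sine.
; The move does not sweep for collision.
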(event EventBeginPlay
  (Variables|Default|SetOriginalPosition (Transformation|GetWorldLocation (Variables|Components|GetPillar))))

(event Collision|EventActorBeginOverlap
  (params (OtherActor :type Actor%20Object%20Reference)))

(event EventTick
  (params (DeltaSeconds :type Float%20%28single-precision%29))
  (bind _returnvalue (Utilities|Time|GetGameTimeinSeconds))
  (bind _frequency (Variables|Default|GetFrequency))
  (bind _amplitude (Variables|Default|Getamplitude))
  (bind _shakexyz (Variables|Default|GetShakeXYZ))
  (bind _returnvalue_2 (* _frequency _returnvalue))
  (bind (_x _y _z) (Math|Vector|BreakVector _shakexyz))
  (bind _returnvalue_3 (Math|Trig|Sin(Radians) _returnvalue_2))
  (bind _returnvalue_4 (* _amplitude _returnvalue_3))
  (Transformation|SetWorldLocation (Variables|Components|GetPillar) (+ (Math|Vector|MakeVector (* _returnvalue_4 _x) (* _y _returnvalue_4) _z) (Variables|Default|GetOriginalPosition)) false false))

(fn ConstructionScript)