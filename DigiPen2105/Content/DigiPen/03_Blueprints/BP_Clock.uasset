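; BP_Clock is an analog clock actor that shows the machine's current time.
; Every tick it reads Now() and sets the relative yaw of the hour, minute and second hand components.
; Each hand adds the fraction of its next smaller unit, so the hands sweep smoothly instead of jumping.
; The construction script runs the same update, so the hands also show the time when the actor is constructed.
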(event Custom|Update_Current_Time
  (bind _returnvalue (Math|DateTime|Now))
  (Variables|Default|SetHour (.hour _returnvalue))
  (Variables|Default|SetMinute (.minute _returnvalue))
  (Variables|Default|SetSecond (.second _returnvalue))
  (Variables|Default|SetMillisecond (.millisecond _returnvalue))
  (Transformation|SetRelativeRotation (Variables|Default|GetHourHand) (Math|Rotator|MakeRotator 0.0 0.0 (+ (* (Variables|Default|GetHour) 3e+01) (* (Variables|Default|GetMinute) 0.5))) false false)
  (Transformation|SetRelativeRotation (Variables|Default|GetMinuteHand) (Math|Rotator|MakeRotator 0.0 0.0 (+ (* (Variables|Default|GetMinute) 6.0) (* (Variables|Default|GetSecond) 0.1))) false false)
  (Transformation|SetRelativeRotation (Variables|Default|GetSecondHand) (Math|Rotator|MakeRotator 0.0 0.0 (+ (* (Variables|Default|GetSecond) 6.0) (* (Variables|Default|GetMillisecond) 0.006))) false false))

(event EventBeginPlay)

(event EventTick
  (params (DeltaSeconds :type Float%20%28single-precision%29))
  (CallFunction|UpdateCurrentTime))

(fn ConstructionScript
  (CallFunction|UpdateCurrentTime))